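; Game mode for Building Escape that runs the menu, timed play and end states and counts down to a loss.
; Tick watches the state enum by name; a change rebuilds widgets, otherwise the timer decrements and sets Lose at zero.
; Each state swaps its widget, input mode, pause and cursor, with End, Win and Lose sharing the score screen.
; That screen first loads and sorts the high-score save, or creates one.
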(event `self.ReceiveBeginPlay`)

(event `self.ReceiveTick`
  (params (DeltaSeconds :type "Float (single-precision)"))
  (set `self.DeltaTime` DeltaSeconds)
  (if (!= (`|GetEnumeratorName` (`self.E_GameState`)) (`self.GameValue`))
    (set `self.GameValue` (`|GetEnumeratorName` (`self.E_GameState`)))
    (`self.ChangeInputAndMouse`)
    (else
      (bind _output_get (set `self.TimeLeft` (- (`self.TimeLeft`) (`self.DeltaTime`))))
      (if (<= _output_get 0.0)
        (set `self.E_GameState` "NewEnumerator4")))))

(fn `ChangeInputAndMouse`
  (switch `/Game/Blueprints/E_GameState` (`self.E_GameState`)
    (:`NewEnumerator0`
      (`self.CreateAllWidgets`))
    (:`NewEnumerator1`
      (`self.CreateAllWidgets`))
    (:`NewEnumerator2`
      (`self.CreateAllWidgets` :!label _label))
    (:`NewEnumerator3`
      (goto _label))
    (:`NewEnumerator4`
      (goto _label))))

(fn `CreateAllWidgets`
  (bind _returnvalue (`GameplayStatics.GetPlayerController` 0))
  (bind _returnvalue_2 (`GameplayStatics.GetPlayerController` 0))
  (bind _returnvalue_3 (`GameplayStatics.GetPlayerController` 0))
  (bind _returnvalue_4 (`GameplayStatics.GetPlayerController` 0))
  (switch `/Game/Blueprints/E_GameState` (`self.E_GameState`)
    (:`NewEnumerator0`
      (`WidgetLayoutLibrary.RemoveAllWidgets`)
      (bind _returnvalue_5 (`|CreateWidget` "/Game/UI/MenWidget.MenWidget_C" _returnvalue_3))
      (`WidgetBlueprintLibrary.SetInputMode_UIOnlyEx` _returnvalue_3 _returnvalue_5)
      (`UserWidget.AddToViewport` _returnvalue_5 0)
      (`GameplayStatics.SetGamePaused` true)
      (set `PlayerController.bShowMouseCursor` true _returnvalue_2)
      (`UserWidget.AddToViewport` _returnvalue_5 0))
    (:`NewEnumerator1`
      (`WidgetLayoutLibrary.RemoveAllWidgets`)
      (bind _returnvalue_6 (`|CreateWidget` "/Game/UI/GameWidget.GameWidget_C" _returnvalue))
      (`WidgetBlueprintLibrary.SetInputMode_GameOnly` _returnvalue)
      (`GameplayStatics.SetGamePaused` false)
      (set `PlayerController.bShowMouseCursor` false _returnvalue_2)
      (`UserWidget.AddToViewport` _returnvalue_6 0))
    (:`NewEnumerator2`
      (`WidgetLayoutLibrary.RemoveAllWidgets` :!label _label)
      (`self.CreateAndLoadGame`)
      (bind _returnvalue_7 (`|CreateWidget` "/Game/UI/ScoreWidget.ScoreWidget_C" _returnvalue_4))
      (`WidgetBlueprintLibrary.SetInputMode_UIOnlyEx` _returnvalue_4 _returnvalue_7)
      (`GameplayStatics.SetGamePaused` true)
      (set `PlayerController.bShowMouseCursor` true _returnvalue_2)
      (`UserWidget.AddToViewport` _returnvalue_7 0))
    (:`NewEnumerator3`
      (goto _label))
    (:`NewEnumerator4`
      (goto _label))))

(fn `CreateAndLoadGame`
  (returns (CurrentSaveObject :type "/Game/Blueprints/BuildingEscape_SaveGame_BP Object Reference"))
  (bind _currentsavegame (`self.CurrentSaveGame`)
    (:`then`
      (return _currentsavegame))
    (:`else`
      (bind _returnvalue (`GameplayStatics.DoesSaveGameExist` (`self.HightScoreSaveName`)))
      (if _returnvalue
        (bind _returnvalue_2 (`GameplayStatics.LoadGameFromSlot` (`self.HightScoreSaveName`)))
        (bind _asbuilding_escape_save_game_bp (cast `/Game/Blueprints/BuildingEscape_SaveGame_BP` _returnvalue_2)
          (:`then`
            (`/Game/Blueprints/BuildingEscape_SaveGame_BP.SortSaveData` _asbuilding_escape_save_game_bp)
            (bind _output_get (set `self.CurrentSaveGame` _asbuilding_escape_save_game_bp))
            (return _output_get))
          (:`CastFailed`
            _))
        (else
          (bind _returnvalue_3 (`GameplayStatics.CreateSaveGameObject` "/Game/Blueprints/BuildingEscape_SaveGame_BP.BuildingEscape_SaveGame_BP_C"))
          (`/Engine/EditorBlueprintResources/StandardMacros.IsValid` _returnvalue_3
            (:`Is Valid`
              (bind _output_get_2 (set `self.CurrentSaveGame` _returnvalue_3))
              (return _output_get_2))
            (:`Is Not Valid`
              _))))
      (return null))))

(fn `UserConstructionScript`)