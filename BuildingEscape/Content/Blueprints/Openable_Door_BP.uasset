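; Openable door for Building Escape, driven by an OpenDoor component's mass-trigger open, close and win events.
; A DoorOpen timeline swings the actor's yaw relative to its starting rotation, plays a lock sound from an event track, and reverses to close.
; It feeds the required mass at BeginPlay and the current total mass every Tick to the game mode, and changes its game state on win.
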(event `self.ReceiveBeginPlay`
  (set `self.IntialRotation` (`self.K2_GetActorRotation`))
  (bind _asbuilding_escape_game_mode_bp (cast `/Game/Blueprints/BuildingEscapeGameMode_BP` (`GameplayStatics.GetGameMode`)))
  (bind _output_get (set `self.GameMode` _asbuilding_escape_game_mode_bp))
  (set `/Game/Blueprints/BuildingEscapeGameMode_BP.TotalMassNeeded` (`OpenDoor.TriggerMassToOpenDoor` (`self.OpenDoor`)) _output_get))

(event `self.OpenDoor.OnOpen`
  (bind (_direction _openangle) (`Timeline|DoorOpen` :`NewTime` 1.0 :!label _label)
    (:`Update`
      (`self.K2_SetActorRotation` (`KismetMathLibrary.ComposeRotators` (`KismetMathLibrary.MakeRotator` 0.0 0.0 _openangle) (`self.IntialRotation`))))
    (:`SoundTiming`
      (`GameplayStatics.PlaySoundAtLocation` "/Game/Sounds/door-lock.door-lock" (`self.K2_GetActorLocation`)))))

(event `self.OpenDoor.OnClose`
  (goto _label :!via `Reverse`))

(event `self.ReceiveTick`
  (params (DeltaSeconds :type "Float (single-precision)"))
  (set `/Game/Blueprints/BuildingEscapeGameMode_BP.WeightLeft` (`OpenDoor.TotalMass` (`self.OpenDoor`)) (`self.GameMode`)))

(event `self.OpenDoor.OnWin`
  (set `/Game/Blueprints/BuildingEscapeGameMode_BP.E_GameState` "NewEnumerator3" (`self.GameMode`)))

(fn `UserConstructionScript`)