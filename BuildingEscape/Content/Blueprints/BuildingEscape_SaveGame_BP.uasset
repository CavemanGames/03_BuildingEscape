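; SaveGame Blueprint for Building Escape that holds the high score table, ranked by time left.
; AddHightScore appends the new entry, sorts the table from most to least time left and trims it to at most six entries.
; SortSaveData is a selection sort that repeatedly moves the highest entry into a temporary array, then copies it back.
; A lowest-score lookup also exists but is not called here.
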(fn `AddHightScore`
  (params (NewScore :type "/Game/Blueprints/HightScoreStructure Structure"))
  (bind _savestructure (`self.SaveStructure`))
  (`KismetArrayLibrary.Array_Add` (`self.SaveStructure`) NewScore)
  (`self.SortSaveData`)
  (`KismetArrayLibrary.Array_Resize` _savestructure (`KismetMathLibrary.Min` 6 (`KismetArrayLibrary.Array_Length` _savestructure))))

(fn `DetermineHighestScoreValue`
  (returns (HighestTimeStruct :type "/Game/Blueprints/HightScoreStructure Structure") (HighestIndexStruct :type Integer))
  (locals (HighestTime :type "Float (double-precision)") (HighestIndex :type Integer))
  (bind _highestindex (`local.HighestIndex`))
  (for (_array_element _array_index) (`self.SaveStructure`)
    (if (== _array_index 0)
      (set `local.HighestTime` (`.TimeLeft_5_F970DAA843846961D06449A2A5AD10B5` (break `/Game/Blueprints/HightScoreStructure` _array_element)))
      (set `local.HighestIndex` _array_index)
      (elif (> (`.TimeLeft_5_F970DAA843846961D06449A2A5AD10B5` (break `/Game/Blueprints/HightScoreStructure` _array_element)) (`local.HighestTime`))
        (set `local.HighestTime` (`.TimeLeft_5_F970DAA843846961D06449A2A5AD10B5` (break `/Game/Blueprints/HightScoreStructure` _array_element)))
        (set `local.HighestIndex` _array_index))))
  (return (`|GetArrayItem` (`self.SaveStructure`) _highestindex) _highestindex))

(fn `DetermineLowestScoreValue`
  (returns (LowestScoreStruct :type "/Game/Blueprints/HightScoreStructure Structure") (LowestScoreIndex :type Integer))
  (locals (LowestTime :type "Float (double-precision)") (LowestIndex :type Integer))
  (bind _lowestindex (`local.LowestIndex`))
  (for (_array_element _array_index) (`self.SaveStructure`)
    (if (== _array_index 0)
      (set `local.LowestTime` (`.TimeLeft_5_F970DAA843846961D06449A2A5AD10B5` (break `/Game/Blueprints/HightScoreStructure` _array_element)))
      (set `local.LowestIndex` _array_index)
      (elif (< (`.TimeLeft_5_F970DAA843846961D06449A2A5AD10B5` (break `/Game/Blueprints/HightScoreStructure` _array_element)) (`local.LowestTime`))
        (set `local.LowestTime` (`.TimeLeft_5_F970DAA843846961D06449A2A5AD10B5` (break `/Game/Blueprints/HightScoreStructure` _array_element)))
        (set `local.LowestIndex` _array_index))))
  (return (`|GetArrayItem` (`self.SaveStructure`) _lowestindex) _lowestindex))

(fn `SortSaveData`
  (locals (TempSaveStruct :type "Array of /Game/Blueprints/HightScoreStructure Structure"))
  (while (> (`KismetArrayLibrary.Array_Length` (`self.SaveStructure`)) 0)
    (bind (_highesttimestruct _highestindexstruct) (`self.DetermineHighestScoreValue`))
    (`KismetArrayLibrary.Array_Add` (`local.TempSaveStruct`) _highesttimestruct)
    (`KismetArrayLibrary.Array_Remove` (`self.SaveStructure`) _highestindexstruct))
  (set `self.SaveStructure` (`local.TempSaveStruct`)))